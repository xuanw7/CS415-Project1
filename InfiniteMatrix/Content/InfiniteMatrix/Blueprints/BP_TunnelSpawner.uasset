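; Spawner actor that builds the endless chain of BP_Tunnel segments and raises difficulty as the tunnel count grows.
; On BeginPlay it clears existing tunnels and health packs, then seeds a few segments from the player's location.
; Each segment attaches at the newest one's SpawnPoint, gets randomized walls and a reference back to the spawner.
; Past the opening segments it randomly scatters enemies and health packs, and each spawn calls SpeedUp on the player, scaled by count.
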(event `self.ReceiveBeginPlay`
  (`self.Spawn Initial Tunnels`))

(fn `Spawn Initial Tunnels`
  (set `self.CountTunnel` 0)
  (`|ExecutionSequence`
    (:`then_0`
      (bind _outactors (`GameplayStatics.GetAllActorsOfClass` "/Game/InfiniteMatrix/Blueprints/BP_Tunnel.BP_Tunnel_C"))
      (for _array_element _outactors
        (`self.K2_DestroyActor` _array_element)
        (bind _outactors_2 (`GameplayStatics.GetAllActorsOfClass` "/Game/InfiniteMatrix/Blueprints/Health_Pack.Health_Pack_C"))
        (for _array_element_2 _outactors_2
          (`self.K2_DestroyActor` _array_element_2))))
    (:`then_1`
      (for _ (range 3)
        (`/Engine/EditorBlueprintResources/StandardMacros.IsValid` (`self.Newest Tunnel`)
          (:`Is Valid`
            (`self.SpawnTunnelAtSpawnPoint`))
          (:`Is Not Valid`
            (`self.SpawnTunnel` (`self.K2_GetActorLocation` (`GameplayStatics.GetPlayerPawn` 0)))))))))

(fn `SpawnTunnel`
  (params (SpawnlLocation :type "Vector Structure"))
  (bind _returnvalue (`|SpawnActorFromClass` "/Game/InfiniteMatrix/Blueprints/BP_Tunnel.BP_Tunnel_C" (`KismetMathLibrary.MakeTransform` SpawnlLocation) "Undefined" "OverrideRootScale" null null))
  (bind _output_get (set `self.Newest Tunnel` _returnvalue))
  (set `/Game/InfiniteMatrix/Blueprints/BP_Tunnel.TunnelSpawner` self _output_get)
  (`/Game/InfiniteMatrix/Blueprints/BP_Tunnel.RandomizeWall` _output_get)
  (`|ExecutionSequence`
    (:`then_0`
      (bind _output_get_2 (set `self.CountTunnel` (+ (`self.CountTunnel`) 1)))
      (if (and (> _output_get_2 5) (== (`KismetMathLibrary.RandomIntegerInRange` 0 4) 0))
        (bind _returnvalue_2 (`|SpawnActorFromClass` "/Game/InfiniteMatrix/Blueprints/Health_Pack.Health_Pack_C" (`KismetMathLibrary.MakeTransform` (+ SpawnlLocation (`KismetMathLibrary.MakeVector` (`KismetMathLibrary.Conv_IntToDouble` (`KismetMathLibrary.RandomIntegerInRange` 500 2000)) (`KismetMathLibrary.Conv_IntToDouble` (`KismetMathLibrary.RandomIntegerInRange` -250 250)) (`KismetMathLibrary.Conv_IntToDouble` (`KismetMathLibrary.RandomIntegerInRange` -250 250))))) "Undefined" "OverrideRootScale" null null))
        (set `/Game/InfiniteMatrix/Blueprints/BP_Tunnel.HealthPack` _returnvalue_2 _returnvalue)))
    (:`then_1`
      (if (> _output_get_2 4)
        (for _ (range 5)
          (if (== (`KismetMathLibrary.RandomIntegerInRange` 0 3) 0)
            (`|SpawnActorFromClass` "/Game/InfiniteMatrix/Blueprints/Enemy.Enemy_C" (`KismetMathLibrary.MakeTransform` (+ SpawnlLocation (`KismetMathLibrary.MakeVector` (`KismetMathLibrary.Conv_IntToDouble` (`KismetMathLibrary.RandomIntegerInRange` 500 2000)) (`KismetMathLibrary.Conv_IntToDouble` (`KismetMathLibrary.RandomIntegerInRange` -250 250)) (`KismetMathLibrary.Conv_IntToDouble` (`KismetMathLibrary.RandomIntegerInRange` -250 250))))) "Undefined" "OverrideRootScale" null null)))))
    (:`then_2`
      (bind _asbp_player (cast `/Game/InfiniteMatrix/Blueprints/BP_Player` (`GameplayStatics.GetPlayerPawn` 0)))
      (`/Game/InfiniteMatrix/Blueprints/BP_Player.SpeedUp` _asbp_player (`KismetMathLibrary.Conv_IntToDouble` (* (/ (`self.CountTunnel`) 5) 25))))))

(fn `SpawnTunnelAtSpawnPoint`
  (locals (NewLocalVar_0 :type "/Game/InfiniteMatrix/Blueprints/BP_Tunnel Object Reference"))
  (`self.SpawnTunnel` (`SceneComponent.K2_GetComponentLocation` (`/Game/InfiniteMatrix/Blueprints/BP_Tunnel.SpawnPoint` (`self.Newest Tunnel`)))))

(fn `UserConstructionScript`)