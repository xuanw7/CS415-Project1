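; Short-lived projectile actor that expires one second after spawning.
; When its Box stops overlapping any actor other than BP_Player, it destroys itself, reacting to end rather than begin overlap.
; ProjectileMovement takes its initial speed from the ProjectileSpeed variable when the component activates.
; The construction script restricts the PointLight to lighting channel 1.
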(event `self.ReceiveBeginPlay`
  (`self.SetLifeSpan` 1.0))

(event `self.Box.OnComponentEndOverlap`
  (params (OverlappedComponent :type "PrimitiveComponent Object Reference") (OtherActor :type "Actor Object Reference") (OtherComp :type "PrimitiveComponent Object Reference") (OtherBodyIndex :type Integer))
  (cast `/Game/InfiniteMatrix/Blueprints/BP_Player` OtherActor
    (:`CastFailed`
      (`self.K2_DestroyActor`))))

(event `self.ProjectileMovement.OnComponentActivated`
  (params (Component :type "ActorComponent Object Reference") (bReset :type Boolean))
  (set `ProjectileMovementComponent.InitialSpeed` (`self.ProjectileSpeed`) (`self.ProjectileMovement`)))

(fn `UserConstructionScript`
  (`LightComponent.SetLightingChannels` (`self.PointLight`) false true false))