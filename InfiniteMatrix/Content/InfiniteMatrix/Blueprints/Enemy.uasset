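; Enemy actor that lives for a limited time and responds to whatever overlaps its Box component.
; A chain of casts sorts the overlapping actor: a health pack or another enemy simply destroys this enemy.
; A projectile hit adds score to the player pawn before the enemy is destroyed.
; Contact with BP_Player reduces health and score, refreshes the displayed score, then destroys the enemy.
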(event `self.ReceiveBeginPlay`
  (`self.SetLifeSpan` 10.0))

(event `self.Box.OnComponentBeginOverlap`
  (params (OverlappedComponent :type "PrimitiveComponent Object Reference") (OtherActor :type "Actor Object Reference") (OtherComp :type "PrimitiveComponent Object Reference") (OtherBodyIndex :type Integer) (bFromSweep :type Boolean) (SweepResult :type "HitResult Structure (by ref)"))
  (cast `/Game/InfiniteMatrix/Blueprints/Health_Pack` OtherActor
    (:`then`
      (`self.K2_DestroyActor`))
    (:`CastFailed`
      (cast `/Game/InfiniteMatrix/Blueprints/Enemy` OtherActor
        (:`then`
          (`self.K2_DestroyActor`))
        (:`CastFailed`
          (cast `/Game/InfiniteMatrix/Blueprints/projectile` OtherActor
            (:`then`
              (bind _asbp_player (cast `/Game/InfiniteMatrix/Blueprints/BP_Player` (`GameplayStatics.GetPlayerPawn` 0)))
              (`/Game/InfiniteMatrix/Blueprints/BP_Player.IncreaseScore` _asbp_player 25)
              (`/Game/InfiniteMatrix/Blueprints/BP_Player.UpdateScoreShown` _asbp_player)
              (`self.K2_DestroyActor`))
            (:`CastFailed`
              (bind _asbp_player_2 (cast `/Game/InfiniteMatrix/Blueprints/BP_Player` OtherActor))
              (`/Game/InfiniteMatrix/Blueprints/BP_Player.ReduceHealth` _asbp_player_2 20)
              (`/Game/InfiniteMatrix/Blueprints/BP_Player.ReduceScore` _asbp_player_2 50)
              (`/Game/InfiniteMatrix/Blueprints/BP_Player.UpdateScoreShown` _asbp_player_2)
              (`self.K2_DestroyActor`))))))))

(fn `UserConstructionScript`)